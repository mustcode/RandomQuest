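; SkillCommandHandler interprets a list of skill commands on behalf of its owner, spawning Skill actors aimed at targets.
; ProcessCommands logs the list through CustomGameMode, then walks it by index, with each handler consuming the following entry as its argument.
; SpawnCommand uses the game mode's ActorSpawner to create named skills per target or one at their average position.
; SetTargetCommand has empty selection branches, leaving Targets unchanged.
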(event EventTick
  (params (DeltaSeconds :type Float%20%28single-precision%29)))

(event EventBeginPlay)

(fn ProcessCommands
  (params (commands :type Array%20of%20Skill%20Command%20Structures))
  (CallFunction|LogCommands commands)
  (LocalVariables|SetcommandIndex 0)
  (while (< (LocalVariables|GetcommandIndex) (Utilities|Array|Length commands))
    (switch name (.command (Utilities|Struct|BreakSkillCommand (Utilities|Array|Get(acopy) commands (LocalVariables|GetcommandIndex))))
      (:Default
        _)
      (:SetTarget
        (bind _newindex (CallFunction|SetTargetCommand commands (LocalVariables|GetcommandIndex)))
        (LocalVariables|SetcommandIndex _newindex))
      (:SpawnForEachTarget
        (bind _newindex_2 (CallFunction|SpawnCommand commands (LocalVariables|GetcommandIndex) true))
        (LocalVariables|SetcommandIndex _newindex_2))
      (:SpawnForAllTargets
        (bind _newindex_3 (CallFunction|SpawnCommand commands (LocalVariables|GetcommandIndex) false))
        (LocalVariables|SetcommandIndex _newindex_3)))
    (Math|Integer|IncrementInt (LocalVariables|GetcommandIndex))))

(fn LogCommands
  (params (commands :type Array%20of%20Skill%20Command%20Structures))
  (bind _ascustom_game_mode (Utilities|Casting|CastToCustomGameMode (Game|GetGameMode)))
  (for _array_element commands
    (Default|LogGameMessage _ascustom_game_mode (Utilities|String|Append (Utilities|String|ToString(Float) (.time (Utilities|Struct|BreakSkillCommand _array_element))) " - " (Utilities|String|ToString(Name) (.command (Utilities|Struct|BreakSkillCommand _array_element))) "(" (Utilities|String|ToString(Float) (.value (Utilities|Struct|BreakSkillCommand _array_element))) ")"))))

(fn SpawnCommand
  (params (commands :type Array%20of%20Skill%20Command%20Structures) (commandIndex :type Integer) (forEachTarget :type Boolean))
  (bind _returnvalue (Game|GetGameMode))
  (bind _result (Math|Integer|IncrementInt commandIndex)
    (:%20%20
      (bind _output_get (LocalVariables|SetcurrentIndex _result))
      (LocalVariables|SetskillName (.command (Utilities|Struct|BreakSkillCommand (Utilities|Array|Get(acopy) commands _output_get))))
      (if forEachTarget
        (bind _ascustom_game_mode (Utilities|Casting|CastToCustomGameMode _returnvalue))
        (for _array_element (Variables|Default|Gettargets)
          (bind _actor (Default|SpawnActor (Variables|/Game/Blueprints/CustomGameMode.CustomGameMode_C|GetActorSpawner _ascustom_game_mode) (LocalVariables|GetskillName) (Math|Transform|MakeTransform (Transformation|GetActorLocation _array_element))))
          (bind _asskill (Utilities|Casting|CastToSkill _actor))
          (Variables|/Game/Blueprints/Skills/Skill.Skill_C|Setactivator _asskill (Components|GetOwner))
          (Utilities|Array|Add (Variables|/Game/Blueprints/Skills/Skill.Skill_C|GettargetActors _asskill) _array_element)
          (Utilities|Array|Add (Variables|Default|Getskill) _asskill))
        (else
          (bind _ascustom_game_mode_2 (Utilities|Casting|CastToCustomGameMode _returnvalue))
          (bind _actor_2 (Default|SpawnActor (Variables|/Game/Blueprints/CustomGameMode.CustomGameMode_C|GetActorSpawner _ascustom_game_mode_2) (LocalVariables|GetskillName) (Math|Transform|MakeTransform (CallFunction|AverageTargetPositions))))
          (bind _asskill_2 (Utilities|Casting|CastToSkill _actor_2))
          (Variables|/Game/Blueprints/Skills/Skill.Skill_C|Setactivator _asskill_2 (Components|GetOwner))
          (for _array_element_2 (Variables|Default|Gettargets)
            (Utilities|Array|Add (Variables|/Game/Blueprints/Skills/Skill.Skill_C|GettargetActors _asskill_2) _array_element_2))
          (Utilities|Array|Add (Variables|Default|Getskill) _asskill_2)))
      (return (LocalVariables|GetcurrentIndex)))))

(fn SetTargetCommand
  (params (commands :type Array%20of%20Skill%20Command%20Structures) (commandIndex :type Integer))
  (bind _result (Math|Integer|IncrementInt commandIndex)
    (:%20%20
      (bind _output_get (LocalVariables|SetcurrentIndex _result))
      (LocalVariables|Setcount (Math|Float|Truncate (.value (Utilities|Struct|BreakSkillCommand (Utilities|Array|Get(acopy) commands _output_get)))))
      (switch name (.command (Utilities|Struct|BreakSkillCommand (Utilities|Array|Get(acopy) commands _output_get)))
        (:Default
          _)
        (:FromFront
          _)
        (:FromBack
          _)
        (:FromCenter
          _))
      (return (LocalVariables|GetcurrentIndex)))))

(fn AverageTargetPositions
  (LocalVariables|SettargetPosition "0, 0, 0")
  (if (> (Utilities|Array|Length (Variables|Default|Gettargets)) 0)
    (for _array_element (Variables|Default|Gettargets)
      (LocalVariables|SettargetPosition (+ (Transformation|GetActorLocation _array_element) (LocalVariables|GettargetPosition))))
    (LocalVariables|SettargetPosition (/ (LocalVariables|GettargetPosition) (Math|Conversions|ToFloat(Integer) (Utilities|Array|Length (Variables|Default|Gettargets))))))
  (return (LocalVariables|GettargetPosition)))