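; Enemy is a combat character Blueprint that sets itself up from game data and faces the hero when play begins.
; On BeginPlay it creates its character through the WorldDataInstance game instance, initializes with it, spawns its default controller, and rotates once toward the first Hero actor found.
; Healed and damaged events pass the amount and critical flag to the CustomPlayerController, which adds status text for the enemy.
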(event `self.ReceiveBeginPlay`
  (bind _asworld_data_instance (cast `WorldDataInstance` (`GameplayStatics.GetGameInstance`)))
  (bind _returnvalue (`WorldDataInstance.CreateCharacter` _asworld_data_instance))
  (`self.Init` _returnvalue)
  (`self.SpawnDefaultController`)
  (`self.TurnToHero`))

(event `self.ReceiveTick`
  (params (DeltaSeconds :type "Float (single-precision)")))

(event `self.OnHealed`
  (params (healer :type "BaseCharacter Object Reference") (amount :type Integer) (isCritical :type Boolean) (healingType :type Name))
  (bind _ascustom_player_controller (cast `/Game/Blueprints/CustomPlayerController` (`GameplayStatics.GetPlayerController` 0)))
  (`/Game/Blueprints/CustomPlayerController.AddStatusText` _ascustom_player_controller self "NewEnumerator0" amount "" isCritical))

(event `self.OnDamaged`
  (params (originator :type "BaseCharacter Object Reference") (amount :type Integer) (isCritical :type Boolean) (damageType :type Name))
  (bind _ascustom_player_controller (cast `/Game/Blueprints/CustomPlayerController` (`GameplayStatics.GetPlayerController` 0)))
  (`/Game/Blueprints/CustomPlayerController.AddStatusText` _ascustom_player_controller self "NewEnumerator1" amount "" isCritical))

(fn `TurnToHero`
  (bind _outactors (`GameplayStatics.GetAllActorsOfClass` "/Game/Blueprints/Hero.Hero_C"))
  (`self.SetActorRotation` (`KismetMathLibrary.FindLookAtRotation` (`self.K2_GetActorLocation`) (`self.K2_GetActorLocation` (`KismetArrayLibrary.Array_Get` _outactors)))))

(fn `UserConstructionScript`)