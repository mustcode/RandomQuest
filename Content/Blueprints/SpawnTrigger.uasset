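; Spawn trigger logic that spawns random actors at its spawn points when a hero enters the owning trigger.
; On BeginPlay it casts its owner to TriggerBase and binds to that actor's begin-overlap event, doing nothing further if the cast fails.
; When the overlapping actor is a Hero or subclass, it loops through SpawnPoints and calls SpawnRandomActor on each one that reports it can spawn.
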(event `self.ReceiveBeginPlay`
  (bind _astrigger_base (cast `TriggerBase` (`self.GetOwner`)))
  (add `Actor.OnActorBeginOverlap` _astrigger_base (delegate `OnActorBeginOverlapped`)))

(event `OnActorBeginOverlapped`
  (params (OtherActor :type "Actor Object Reference"))
  (if (`KismetMathLibrary.ClassIsChildOf` (`GameplayStatics.GetObjectClass` OtherActor) "/Game/Blueprints/Hero.Hero_C")
    (for _array_element (`self.SpawnPoints`)
      (if (`/Game/Blueprints/RandomActorSpawnPoint.CanSpawn` _array_element)
        (`/Game/Blueprints/RandomActorSpawnPoint.SpawnRandomActor` _array_element)))))