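; Base logic for an interactable town structure that the player can enter after confirming a prompt.
; On BeginPlay it creates and initializes a data entry under the current town in WorldDataInstance if none exists for its name.
; Interacting opens the player controller's confirm dialog, unless one is already visible.
; Confirming calls OnEnterBuilding, which cuts instantly to the interior camera rather than moving the player.
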(event `self.ReceiveBeginPlay`
  (`|ExecutionSequence`
    (:`then_0`
      (bind _asworld_data_instance (cast `WorldDataInstance` (`GameplayStatics.GetGameInstance`)))
      (bind _returnvalue (`WorldDataInstance.GetCurrentTown` _asworld_data_instance))
      (if (!= _returnvalue null)
        (if (not (`LocationObject.HasChild` _returnvalue (`self.StructureName`)))
          (`self.Init` (`WorldDataInstance.CreateStructure` _asworld_data_instance (`self.StructureName`) (`self.StructureType`) _returnvalue)))))
    (:`then_1`
      (add `/Game/Blueprints/Interactable.OnInteract` (`self.Interactable`) (delegate `OnInteract`)))))

(event `OnInteract`
  (`KismetSystemLibrary.PrintString` (`KismetStringLibrary.Conv_NameToString` (`self.StructureName`)))
  (bind _ascustom_player_controller (cast `/Game/Blueprints/CustomPlayerController` (`GameplayStatics.GetPlayerController` 0)))
  (bind _isvisible (`/Game/Blueprints/CustomPlayerController.IsConfirmDialogVisible` _ascustom_player_controller))
  (if (not _isvisible)
    (bind _dialogbox (`/Game/Blueprints/CustomPlayerController.OpenConfirmDialog` _ascustom_player_controller (`KismetTextLibrary.Conv_StringToText` (`KismetStringLibrary.BuildString_Name` "" "Enter " (`self.StructureName`) "?")) "Yes" "No"))
    (add `/Game/Widgets/ConfirmDialogBox.OnConfirm` _dialogbox (delegate `OnConfirm`))))

(event `OnConfirm`
  (`self.OnEnterBuilding`))

(fn `OnEnterBuilding`
  (returns (success :type Boolean))
  (`KismetSystemLibrary.PrintString` (`KismetStringLibrary.Concat_StrStr` "You're inside " (`KismetStringLibrary.Conv_NameToString` (`self.StructureName`))))
  (bind _ascustom_player_controller (cast `/Game/Blueprints/CustomPlayerController` (`GameplayStatics.GetPlayerController` 0)))
  (`/Game/Blueprints/CustomPlayerController.SetCurrentCamera` _ascustom_player_controller (`self.InsideCamera`) 0.0)
  (return true))

(fn `UserConstructionScript`)