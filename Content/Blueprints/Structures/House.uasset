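; House is a structure Blueprint for a building, derived from a parent structure class.
; Its construction script runs the parent's, then labels a TextRender component with StructureName, falling back to StructureType when the name is None.
; OnEnterBuilding only forwards to the parent implementation and returns its result, adding no house-specific behavior.
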(fn `OnEnterBuilding`
  (returns (success :type Boolean))
  (bind _success (`parent.OnEnterBuilding`))
  (return _success))

(fn `UserConstructionScript`
  (bind _textrender (`self.TextRender`))
  (`parent.UserConstructionScript`)
  (if (!= (`self.StructureName`) "None")
    (`TextRenderComponent.SetText` _textrender (`KismetStringLibrary.Conv_NameToString` (`self.StructureName`)))
    (else
      (`TextRenderComponent.SetText` _textrender (`KismetStringLibrary.Conv_NameToString` (`self.StructureType`))))))