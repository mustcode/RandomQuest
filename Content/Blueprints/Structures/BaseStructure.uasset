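; Base Blueprint for a clickable town structure that the player can enter.
; On BeginPlay it creates and initializes structure data under the WorldDataInstance's current town if that town has no child with its name.
; A click and release opens the CustomPlayerController's confirm dialog unless one is already visible.
; Confirming calls OnEnterBuilding, which cuts the controller's camera to the structure's inside camera.
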(event `self.ReceiveBeginPlay`
  (bind _asworld_data_instance (cast `WorldDataInstance` (`GameplayStatics.GetGameInstance`)))
  (bind _returnvalue (`WorldDataInstance.GetCurrentTown` _asworld_data_instance))
  (if (!= _returnvalue null)
    (if (not (`LocationObject.HasChild` _returnvalue (`self.StructureName`)))
      (`self.Init` (`WorldDataInstance.CreateStructure` _asworld_data_instance (`self.StructureName`) (`self.StructureType`) _returnvalue)))))

(event `self.ReceiveActorOnClicked`
  (set `self.clicked` true))

(event `self.ReceiveActorOnReleased`
  (if (`self.clicked`)
    (set `self.clicked` false)
    (`KismetSystemLibrary.PrintString` (`KismetStringLibrary.Conv_NameToString` (`self.StructureName`)))
    (bind _ascustom_player_controller (cast `/Game/Blueprints/CustomPlayerController` (`GameplayStatics.GetPlayerController` 0)))
    (bind _isvisible (`/Game/Blueprints/CustomPlayerController.IsConfirmDialogVisible` _ascustom_player_controller))
    (if (not _isvisible)
      (bind _dialogbox (`/Game/Blueprints/CustomPlayerController.OpenConfirmDialog` _ascustom_player_controller (`KismetTextLibrary.Conv_StringToText` (`KismetStringLibrary.BuildString_Name` "" "Enter " (`self.StructureName`) "?")) "Yes" "No"))
      (add `/Game/Widgets/ConfirmDialogBox.OnConfirm` _dialogbox (delegate `OnConfirm`)))))

(event `OnConfirm`
  (`self.OnEnterBuilding`))

(fn `OnEnterBuilding`
  (returns (success :type Boolean))
  (`KismetSystemLibrary.PrintString` (`KismetStringLibrary.Concat_StrStr` "You're inside " (`KismetStringLibrary.Conv_NameToString` (`self.StructureName`))))
  (bind _ascustom_player_controller (cast `/Game/Blueprints/CustomPlayerController` (`GameplayStatics.GetPlayerController` 0)))
  (`/Game/Blueprints/CustomPlayerController.SetCurrentCamera` _ascustom_player_controller (`self.InsideCamera`) 0.0)
  (return true))

(fn `UserConstructionScript`)