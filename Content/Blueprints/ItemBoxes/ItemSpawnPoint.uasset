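; ItemSpawnPoint is a placeable actor that spawns a named item at its own transform.
; SpawnItem asks the CustomGameMode's ItemSpawner to spawn the actor, then has the WorldDataInstance game instance create matching item data.
; It assigns that data to the spawned Item's ItemInstance and returns the Item.
; The event graph and construction script are empty, so spawning only happens when SpawnItem is called.
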(event `self.ReceiveBeginPlay`)

(event `self.ReceiveActorBeginOverlap`
  (params (OtherActor :type "Actor Object Reference")))

(event `self.ReceiveTick`
  (params (DeltaSeconds :type "Float (single-precision)")))

(fn `SpawnItem`
  (params (ItemToSpawn :type Name))
  (returns (item :type "/Game/Blueprints/Items/Item Object Reference"))
  (bind _ascustom_game_mode (cast `/Game/Blueprints/CustomGameMode` (`GameplayStatics.GetGameMode`)))
  (bind _actor (`/Game/Blueprints/ActorSpawner.SpawnActor` (`/Game/Blueprints/CustomGameMode.ItemSpawner` _ascustom_game_mode) ItemToSpawn (`self.GetTransform`)))
  (bind _asworld_data_instance (cast `WorldDataInstance` (`GameplayStatics.GetGameInstance`)))
  (bind _returnvalue (`WorldDataInstance.CreateItem` _asworld_data_instance ItemToSpawn))
  (bind _asitem (cast `/Game/Blueprints/Items/Item` _actor))
  (set `/Game/Blueprints/Items/Item.ItemInstance` _returnvalue _asitem)
  (return _asitem))

(fn `UserConstructionScript`)