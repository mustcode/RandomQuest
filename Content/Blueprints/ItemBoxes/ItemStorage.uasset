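; Interactable storage container that gives the player access to a named inventory.
; On BeginPlay it looks up its inventory by StorageName in the WorldDataInstance game instance, creating one with its space and weight limits if none exists.
; On interact it sets the interact target for all heroes and, unless an inventory widget is already visible, opens one through the player controller's WidgetManager with a close button.
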(event `self.ReceiveBeginPlay`
  (bind _asworld_data_instance (cast `WorldDataInstance` (`GameplayStatics.GetGameInstance`)))
  (bind _output_get (set `self.Inventory` (`WorldDataInstance.GetStorageInventory` _asworld_data_instance (`self.StorageName`))))
  (if (== _output_get null)
    (bind _returnvalue (`WorldDataInstance.CreateStorageInventory` _asworld_data_instance (`self.StorageName`) (`self.MaxSpace`) (`self.MaxWeight`)))
    (set `self.Inventory` _returnvalue)))

(event `self.Interactable.OnInteract`
  (`/Game/Blueprints/Interactable.SetInteractTargetForAllHeroes` (`self.Interactable`))
  (bind _ascustom_player_controller (cast `/Game/Blueprints/CustomPlayerController` (`GameplayStatics.GetPlayerController` 0)))
  (bind _widgetmanager (`/Game/Blueprints/CustomPlayerController.WidgetManager` _ascustom_player_controller))
  (if (not (`/Game/Blueprints/WidgetManager.IsInventoryWidgetVisible` _widgetmanager))
    (bind _widget (`/Game/Blueprints/WidgetManager.OpenInventoryWidget` _widgetmanager null (`self.Inventory`)))
    (bind _output_get (set `self.InventoryWidget` _widget))
    (`/Game/Widgets/Status/Inventory.ShowCloseButton` _output_get)))

(fn `UserConstructionScript`)