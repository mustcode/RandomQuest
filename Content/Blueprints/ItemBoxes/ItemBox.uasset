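; Interactable item box that spawns random loot once when opened, then refreshes the interact target for all heroes.
; OnOpen rolls each spawnable item against its drop rate and spawns successes at successive spawn points until the list ends or points run out.
; If the count is below the box's minimum, it re-enters the loop to add more items; otherwise it marks the box collected.
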(event OnInteract(Interactable)
  (if (not (Variables|Default|Getcollected))
    (CallFunction|OnOpen)
    (Default|SetInteractTargetforAllHeroes (Variables|Default|GetInteractable))))

(fn ConstructionScript)

(fn OnOpen
  (LocalVariables|SetspawnedItemCount 0)
  (bind _array_element (Utilities|Array|ForEachLoopwithBreak (Variables|Default|GetSpawnableItems) :!label _label)
    (:LoopBody
      (if (>= (.DropRate (Utilities|Struct|BreakSpawnableItem _array_element)) (Math|Random|RandomFloatinRange 0.0 1.0))
        (Default|SpawnItem (Utilities|Array|Get(acopy) (Variables|Default|GetItemSpawnPoints) (LocalVariables|GetspawnedItemCount)) (.ItemClass (Utilities|Struct|BreakSpawnableItem _array_element)))
        (bind _output_get (LocalVariables|SetspawnedItemCount (+ (LocalVariables|GetspawnedItemCount) 1)))
        (if (>= _output_get (Utilities|Array|Length (Variables|Default|GetItemSpawnPoints)))
          (goto _label Break))))
    (:Completed
      (if (< (LocalVariables|GetspawnedItemCount) (Variables|Default|GetMinItemsInBox))
        (goto _label)
        (else
          (Variables|Default|Setcollected true))))))