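; NPC Blueprint that opens a conversation dialog with the player when interacted with.
; On BeginPlay it binds its interaction handler to the Interactable's OnInteract event.
; The handler passes the WorldDataInstance game instance to Dialog's StartConversation.
; If that succeeds, the CustomPlayerController opens the conversation dialog with this NPC as its argument.
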(event `self.ReceiveBeginPlay`
  (add `/Game/Blueprints/Interactable.OnInteract` (`self.Interactable`) (delegate `OnInteract`)))

(event `OnInteract`
  (`KismetSystemLibrary.PrintString` "NPC Clicked")
  (bind _asworld_data_instance (cast `WorldDataInstance` (`GameplayStatics.GetGameInstance`)))
  (bind _returnvalue (`DialogComponent.StartConversation` (`self.Dialog`) _asworld_data_instance))
  (if _returnvalue
    (bind _ascustom_player_controller (cast `/Game/Blueprints/CustomPlayerController` (`GameplayStatics.GetPlayerController` 0)))
    (`/Game/Blueprints/CustomPlayerController.OpenConversationDialog` _ascustom_player_controller self)))

(fn `UserConstructionScript`)