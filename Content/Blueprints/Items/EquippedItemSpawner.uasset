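; EquippedItemSpawner spawns and removes the actors that visually represent items equipped on a character.
; SpawnEquippedItem finds the first Items entry matching the item's name, then spawns an actor for each item part and snaps it to that part's socket on the character's mesh.
; Each spawned actor is registered with the character's EquippedItemsTracker component, to which DestroyEquippedItem delegates removal.
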(event `self.ReceiveBeginPlay`)

(event `self.ReceiveTick`
  (params (DeltaSeconds :type "Float (single-precision)")))

(fn `DestroyEquippedItem`
  (params (item :type "ItemInstanceObject Object Reference") (actor :type "BaseCharacter Object Reference"))
  (`/Game/Blueprints/Items/EquippedItemsTracker.RemoveEquippedItem` (`KismetArrayLibrary.Array_Get` (`Actor.K2_GetComponentsByClass` actor "/Game/Blueprints/Items/EquippedItemsTracker.EquippedItemsTracker_C")) item))

(fn `SpawnEquippedItem`
  (params (item :type "ItemInstanceObject Object Reference") (actor :type "BaseCharacter Object Reference"))
  (for _array_element (`self.items`)
    (bind (_name _itemparts) (break `/Game/Blueprints/Items/EquippedItemVisual` _array_element))
    (if (== _name (`ItemInstanceObject.GetName` item))
      (for _array_element_2 _itemparts
        (bind (_slot _actorclass) (break `/Game/Blueprints/Items/EquippedItemPart` _array_element_2))
        (bind _returnvalue (`|SpawnActorFromClass` _actorclass (`KismetMathLibrary.MakeTransform` (0.0 0.0 0.0)) "AlwaysSpawn" "OverrideRootScale"))
        (`Actor.K2_AttachRootComponentTo` _returnvalue (`Character.Mesh` actor) _slot "SnapToTarget" true)
        (`/Game/Blueprints/Items/EquippedItemsTracker.AddEquippedItemActor` (`KismetArrayLibrary.Array_Get` (`Actor.K2_GetComponentsByClass` actor "/Game/Blueprints/Items/EquippedItemsTracker.EquippedItemsTracker_C")) item _returnvalue))
      (break))))