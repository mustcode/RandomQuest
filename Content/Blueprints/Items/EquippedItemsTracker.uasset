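; Tracks equipped items alongside the actors associated with them, stored as item-actor pairs in an Items array.
; AddEquippedItemActor appends a new pair without checking for duplicates.
; RemoveEquippedItem walks the array from the end so removal by index is safe, destroying the actor and dropping the entry for every match.
; The event graph holds no active logic.
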(event EventBeginPlay)

(event EventTick
  (params (DeltaSeconds :type Float%20%28single-precision%29)))

(fn AddEquippedItemActor
  (params (item :type Item%20Instance%20Object%20Object%20Reference) (actor :type Actor%20Object%20Reference))
  (Utilities|Array|Add (Variables|Default|Getitems) (Utilities|Struct|MakeItemActorPair item actor)))

(fn RemoveEquippedItem
  (params (item :type Item%20Instance%20Object%20Object%20Reference))
  (bind _output_get (LocalVariables|SetlastIndex (- (Utilities|Array|Length (Variables|Default|Getitems)) 1)))
  (for _index (range 0 _output_get)
    (if (== item (.item (Utilities|Struct|BreakItemActorPair (Utilities|Array|Get(acopy) (Variables|Default|Getitems) (- (LocalVariables|GetlastIndex) _index)))))
      (Actor|DestroyActor (.actor (Utilities|Struct|BreakItemActorPair (Utilities|Array|Get(acopy) (Variables|Default|Getitems) (- (LocalVariables|GetlastIndex) _index)))))
      (Utilities|Array|RemoveIndex (Variables|Default|Getitems) (- (LocalVariables|GetlastIndex) _index)))))