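; WidgetManager is a Blueprint that creates and tracks the game's confirm dialog, conversation dialog and skill selection widgets.
; Each open function creates a fresh widget, stores it, adds it to the viewport and returns it, applying supplied text or dialog owner where relevant.
; AdvanceConversation forwards to the conversation dialog when it is visible.
; Null-safe visibility checks per widget combine into IsAnyWidgetVisible, which reports whether any of them is showing.
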(event EventTick
  (params (DeltaSeconds :type Float%20%28single-precision%29)))

(event EventBeginPlay)

(fn OpenConfirmDialog
  (params (QuestionText :type Text) (ConfirmText :type Text) (CancelText :type Text))
  (bind _returnvalue (UserInterface|CreateWidget "/Game/Widgets/ConfirmDialogBox.ConfirmDialogBox_C"))
  (Variables|Default|SetConfirmDIalog _returnvalue)
  (Utilities|FlowControl|Sequence
    (:then_0
      (Variables|/Game/Widgets/ConfirmDialogBox.ConfirmDialogBox_C|SetQuestionText (Variables|Default|GetConfirmDIalog) QuestionText))
    (:then_1
      (Variables|/Game/Widgets/ConfirmDialogBox.ConfirmDialogBox_C|SetConfirmText (Variables|Default|GetConfirmDIalog) ConfirmText))
    (:then_2
      (Variables|/Game/Widgets/ConfirmDialogBox.ConfirmDialogBox_C|SetCancelText (Variables|Default|GetConfirmDIalog) CancelText))
    (:then_3
      (UserInterface|Viewport|AddtoViewport (Variables|Default|GetConfirmDIalog) 0)
      (return (Variables|Default|GetConfirmDIalog)))))

(fn IsConfirmDialogVisible
  (return (CallFunction|IsWidgetVisible (Variables|Default|GetConfirmDialog))))

(fn OpenConversationDialog
  (params (DialogOwner :type Actor%20Object%20Reference))
  (bind _returnvalue (UserInterface|CreateWidget "/Game/Widgets/ConversationDialog.ConversationDialog_C" 0 DialogOwner))
  (bind _output_get (Variables|Default|SetConversationDialog _returnvalue))
  (Default|HideChoices _output_get)
  (UserInterface|Viewport|AddtoViewport (Variables|Default|GetConversationDialog) 0)
  (return (Variables|Default|GetConversationDialog)))

(fn AdvanceConversation
  (if (!= (Variables|Default|GetConversationDialog) 0)
    (if (Widget|IsVisible (Variables|Default|GetConversationDialog))
      (Default|AdvanceConversation (Variables|Default|GetConversationDialog)))))

(fn IsConversationDialogVisible
  (return (CallFunction|IsWidgetVisible (Variables|Default|GetConversationDialog))))

(fn OpenSelectSkillWidget
  (bind _returnvalue (UserInterface|CreateWidget "/Game/Widgets/Skill/SelectSkill.SelectSkill_C"))
  (bind _output_get (Variables|Default|SetSelectSkillWidget _returnvalue))
  (UserInterface|Viewport|AddtoViewport _output_get 0)
  (return _output_get))

(fn IsSelectSkillWidgetVisible
  (return (CallFunction|IsWidgetVisible (Variables|Default|GetSelectSkillWidget))))

(fn IsWidgetVisible
  (params (widget :type Widget%20Object%20Reference))
  (if (!= widget 0)
    (LocalVariables|Setresult (Widget|IsVisible widget))
    (else
      (LocalVariables|Setresult false)))
  (return (LocalVariables|Getresult)))

(fn IsAnyWidgetVisible
  (return (Math|Boolean|ORBoolean (CallFunction|IsConfirmDialogVisible) (CallFunction|IsConversationDialogVisible) (CallFunction|IsSelectSkillWidgetVisible))))