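; GameWorld bootstraps a new game on BeginPlay, loading game data and creating the player's starting state before opening a random starting town.
; LoadDataTables copies skill, trait, occupation, race, equip slot and item tables into GameData, linking skill and trait prerequisites in a second pass after both are registered.
; It then stores an inventory with starter items and gold on the WorldDataInstance and has CustomGameMode add random heroes to the party.
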(event `self.ReceiveBeginPlay`
  (bind _startingtowns (`self.startingTowns`))
  (`self.LoadDataTables`)
  (`|ExecutionSequence`
    (:`then_0`
      (bind _asworld_data_instance (cast `WorldDataInstance` (`GameplayStatics.GetGameInstance`)))
      (bind _returnvalue (`WorldDataInstance.CreateInventory` _asworld_data_instance "Inventory" 100.0 100.0))
      (set `WorldDataInstance.inventory` _returnvalue _asworld_data_instance)
      (`|ExecutionSequence`
        (:`then_0`
          (bind _returnvalue_2 (`WorldDataInstance.CreateItem` _asworld_data_instance "RandomJunk"))
          (`InventoryObject.AddItem` _returnvalue _returnvalue_2))
        (:`then_1`
          (bind _returnvalue_3 (`WorldDataInstance.CreateItem` _asworld_data_instance "BasicArmor"))
          (`InventoryObject.AddItem` _returnvalue _returnvalue_3))
        (:`then_2`
          (`InventoryObject.AddGold` _returnvalue 100))))
    (:`then_1`
      (bind _ascustom_game_mode (cast `/Game/Blueprints/CustomGameMode` (`GameplayStatics.GetGameMode`)))
      (for _ (range 3)
        (`/Game/Blueprints/CustomGameMode.AddRandomHeroToParty` _ascustom_game_mode)))
    (:`then_2`
      (`GameplayStatics.OpenLevel` (`KismetArrayLibrary.Array_Get` _startingtowns (`KismetMathLibrary.RandomInteger` (`KismetArrayLibrary.Array_Length` _startingtowns)))))))

(fn `LoadDataTables`
  (bind _gamedata (`self.GameData`))
  (`|ExecutionSequence`
    (:`then_0`
      (bind _outrownames (`DataTableFunctionLibrary.GetDataTableRowNames` "/Game/DataTables/SkillsTable.SkillsTable"))
      (for _array_element _outrownames
        (bind _returnvalue (`|GetDataTableRow` "/Game/DataTables/SkillsTable.SkillsTable" _array_element)
          (:`then`
            (`GameDataComponent.AddSkill` _gamedata _returnvalue)))))
    (:`then_1`
      (bind _outrownames_2 (`DataTableFunctionLibrary.GetDataTableRowNames` "/Game/DataTables/TraitsTable.TraitsTable"))
      (for _array_element_2 _outrownames_2
        (bind _returnvalue_2 (`|GetDataTableRow` "/Game/DataTables/TraitsTable.TraitsTable" _array_element_2)
          (:`then`
            (`GameDataComponent.AddTrait` _gamedata _returnvalue_2)))))
    (:`then_2`
      (bind _outrownames_3 (`DataTableFunctionLibrary.GetDataTableRowNames` "/Game/DataTables/SkillsTable.SkillsTable"))
      (for _array_element_3 _outrownames_3
        (bind _returnvalue_3 (`|GetDataTableRow` "/Game/DataTables/SkillsTable.SkillsTable" _array_element_3)
          (:`then`
            (bind (_displayname _description _name _variationof _isusableincombat _isusableoutofcombat _canselecttargetally _canselecttargetenemy _commands _costs _prerequisite) (break `Skill` _returnvalue_3))
            (`GameDataComponent.AddPrerequisite` _gamedata _name _prerequisite)))))
    (:`then_3`
      (bind _outrownames_4 (`DataTableFunctionLibrary.GetDataTableRowNames` "/Game/DataTables/TraitsTable.TraitsTable"))
      (for _array_element_4 _outrownames_4
        (bind _returnvalue_4 (`|GetDataTableRow` "/Game/DataTables/TraitsTable.TraitsTable" _array_element_4)
          (:`then`
            (bind (_displayname_2 _description_2 _name_2 _properties _prerequisite_2) (break `Trait` _returnvalue_4))
            (`GameDataComponent.AddPrerequisite` _gamedata _name_2 _prerequisite_2)))))
    (:`then_4`
      (bind _outrownames_5 (`DataTableFunctionLibrary.GetDataTableRowNames` "/Game/DataTables/OccupationsTable.OccupationsTable"))
      (for _array_element_5 _outrownames_5
        (bind _returnvalue_5 (`|GetDataTableRow` "/Game/DataTables/OccupationsTable.OccupationsTable" _array_element_5)
          (:`then`
            (`GameDataComponent.AddOccupation` _gamedata _returnvalue_5)))))
    (:`then_5`
      (bind _outrownames_6 (`DataTableFunctionLibrary.GetDataTableRowNames` "/Game/DataTables/RacesTable.RacesTable"))
      (for _array_element_6 _outrownames_6
        (bind _returnvalue_6 (`|GetDataTableRow` "/Game/DataTables/RacesTable.RacesTable" _array_element_6)
          (:`then`
            (`GameDataComponent.AddRace` _gamedata _returnvalue_6)))))
    (:`then_6`
      (bind _outrownames_7 (`DataTableFunctionLibrary.GetDataTableRowNames` "/Game/DataTables/EquipSlotsTable.EquipSlotsTable"))
      (for _array_element_7 _outrownames_7
        (bind _returnvalue_7 (`|GetDataTableRow` "/Game/DataTables/EquipSlotsTable.EquipSlotsTable" _array_element_7)
          (:`then`
            (`GameDataComponent.AddEquipSlot` _gamedata _returnvalue_7)))))
    (:`then_7`
      (bind _outrownames_8 (`DataTableFunctionLibrary.GetDataTableRowNames` "/Game/DataTables/ItemsTable.ItemsTable"))
      (for _array_element_8 _outrownames_8
        (bind _returnvalue_8 (`|GetDataTableRow` "/Game/DataTables/ItemsTable.ItemsTable" _array_element_8)
          (:`then`
            (`GameDataComponent.AddItem` _gamedata _returnvalue_8)))))))

(fn `UserConstructionScript`)