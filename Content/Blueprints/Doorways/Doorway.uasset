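; Doorway actor with a sign whose door swings open while the mouse cursor hovers over its box.
; The DoorOpen timeline adds yaw from its Speed track, scaled by a delta time cached in Tick.
; Cursor exit snaps the door shut unless CustomPlayerController shows a dialog box, and OnCloseConfirmDialog also resets it.
; The construction script writes the Sign value to the text render.
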(event `self.ReceiveTick`
  (params (DeltaSeconds :type "Float (single-precision)"))
  (set `self.deltaSeconds` DeltaSeconds))

(event `self.Box.OnBeginCursorOver`
  (params (TouchedComponent :type "PrimitiveComponent Object Reference"))
  (`SceneComponent.K2_SetRelativeRotation` :`self` (`self.DoorMesh`))
  (bind (_direction _speed) (`Timeline|DoorOpen` :!via `PlayFromStart`)
    (:`Update`
      (`SceneComponent.K2_AddRelativeRotation` (`self.DoorMesh`) (`KismetMathLibrary.MakeRot` 0.0 (* _speed (* (`self.deltaSeconds`) 200.0))) false))))

(event `self.Box.OnEndCursorOver`
  (params (TouchedComponent :type "PrimitiveComponent Object Reference"))
  (bind _ascustom_player_controller (cast `/Game/Blueprints/CustomPlayerController` (`GameplayStatics.GetPlayerController` 0)))
  (bind _isvisible (`/Game/Blueprints/CustomPlayerController.IsAnyDialogBoxVisible` _ascustom_player_controller))
  (if (not _isvisible)
    (`SceneComponent.K2_SetRelativeRotation` :`self` (`self.DoorMesh`))))

(event `self.OnCloseConfirmDialog`
  (`SceneComponent.K2_SetRelativeRotation` :`self` (`self.DoorMesh`)))

(fn `UserConstructionScript`
  (`parent.UserConstructionScript`)
  (`TextRenderComponent.SetText` (`self.TextRender`) (`KismetTextLibrary.Conv_TextToString` (`self.Sign`))))