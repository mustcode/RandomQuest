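; One-way doorway that, after a Yes/No confirmation, switches the camera and teleports the heroes to its exit points.
; Interacting opens the confirm dialog unless another dialog is visible, then sets the interact target for all heroes.
; Confirming cuts to the target camera and places each Hero at the exit point matching its WorldDataInstance character index.
; The dialog close handler only prints whether the door was entered.
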(event `self.ReceiveBeginPlay`
  (add `/Game/Blueprints/Interactable.OnInteract` (`self.Interactable`) (delegate `OnInteract`)))

(event `OnInteract`
  (`|ExecutionSequence`
    (:`then_0`
      (bind _ascustom_player_controller (cast `/Game/Blueprints/CustomPlayerController` (`GameplayStatics.GetPlayerController` 0)))
      (bind _isvisible (`/Game/Blueprints/CustomPlayerController.IsAnyDialogBoxVisible` _ascustom_player_controller))
      (if (not _isvisible)
        (bind _dialogbox (`/Game/Blueprints/CustomPlayerController.OpenConfirmDialog` _ascustom_player_controller (`self.ConfirmMessage`) "Yes" "No"))
        (add `/Game/Widgets/ConfirmDialogBox.OnConfirm` _dialogbox (delegate `OnConfirm`))
        (add `/Game/Widgets/ConfirmDialogBox.OnCancel` _dialogbox (delegate `OnCancel`))))
    (:`then_1`
      (`/Game/Blueprints/Interactable.SetInteractTargetForAllHeroes` (`self.Interactable`)))))

(event `OnCancel`
  (`self.OnCloseConfirmDialog` false))

(event `OnConfirm`
  (`/Game/Blueprints/CustomPlayerController.SetCurrentCamera` (stale `OnInteract` _ascustom_player_controller) (`self.SwitchToCamera`) 0.0)
  (if (> (`KismetArrayLibrary.Array_Length` (`self.ExitPoints`)) 0)
    (`self.MoveHeroesToExitPoints`))
  (`self.OnCloseConfirmDialog` true))

(fn `MoveHeroesToExitPoints`
  (bind _asworld_data_instance (cast `WorldDataInstance` (`GameplayStatics.GetGameInstance`)))
  (bind _outactors (`GameplayStatics.GetAllActorsOfClass` "/Game/Blueprints/Hero.Hero_C"))
  (for _array_element _outactors
    (bind _returnvalue (`WorldDataInstance.GetCharacterIndex` _asworld_data_instance (`BaseCharacter.character` _array_element)))
    (`self.K2_SetActorLocation` _array_element (`self.K2_GetActorLocation` (`KismetArrayLibrary.Array_Get` (`self.ExitPoints`) _returnvalue)) false)))

(fn `OnCloseConfirmDialog`
  (params (DidEnterDoor :type Boolean))
  (if DidEnterDoor
    (`KismetSystemLibrary.PrintString` "Enter door")
    (else
      (`KismetSystemLibrary.PrintString` "Cancel enter door"))))

(fn `UserConstructionScript`)