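; Dungeon doorway that lets the player attempt to get past its lock through dialog and an ability test.
; When locked, it starts its Dialog conversation and opens the conversation widget through the player controller.
; A decision hides the conversation and opens a Strength test for TryBreak, otherwise a Dexterity test.
; Success clears IsLocked, and success, failure or cancel each picks a dialog choice and shows the conversation again.
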(event `self.OnDoorLocked`
  (bind _ascustom_player_controller (cast `/Game/Blueprints/CustomPlayerController` (`GameplayStatics.GetPlayerController` 0)))
  (bind _asworld_data_instance (cast `WorldDataInstance` (`GameplayStatics.GetGameInstance`)))
  (bind _returnvalue (`DialogComponent.StartConversation` (`self.Dialog`) _asworld_data_instance))
  (if _returnvalue
    (bind _dialogbox (`/Game/Blueprints/CustomPlayerController.OpenConversationDialog` _ascustom_player_controller self))
    (bind _output_get (set `self.ConversationDialog` _dialogbox))
    (add `/Game/Widgets/ConversationDialog.OnMakeDecision` _output_get (delegate `OnMakeDecision`))))

(event `OnMakeDecision`
  (params (conversation :type "Conversation Structure"))
  (`Widget.SetVisibility` (`self.ConversationDialog`) "Hidden")
  (if (== (`.name` (break `Conversation` conversation)) "TryBreak")
    (bind _dialogbox (`/Game/Blueprints/CustomPlayerController.OpenAbilityTestDialog` (stale `self.OnDoorLocked` _ascustom_player_controller) "STR" 3))
    (set `self.AbilityTestWidget` _dialogbox)
    (else
      (bind _dialogbox_2 (`/Game/Blueprints/CustomPlayerController.OpenAbilityTestDialog` (stale `self.OnDoorLocked` _ascustom_player_controller) "DEX" 3))
      (set `self.AbilityTestWidget` _dialogbox_2)))
  (add `/Game/Widgets/AbilityTest.OnCancel` (`self.AbilityTestWidget`) (delegate `OnCancelAbilityTest`))
  (add `/Game/Widgets/AbilityTest.OnClose` (`self.AbilityTestWidget`) (delegate `OnAbilityTestComplete`)))

(event `OnCancelAbilityTest`
  (`/Game/Widgets/ConversationDialog.MakeChoice` (`self.ConversationDialog`) 2)
  (`Widget.SetVisibility` (`self.ConversationDialog`) "Visible" :!label _label))

(event `OnAbilityTestComplete`
  (params (Result :type Boolean) (Rolled :type Integer))
  (set `self.IsLocked` (not Result))
  (if Result
    (`/Game/Widgets/ConversationDialog.MakeChoice` (`self.ConversationDialog`) 0)
    (goto _label)
    (else
      (`/Game/Widgets/ConversationDialog.MakeChoice` (`self.ConversationDialog`) 1)
      (goto _label))))

(fn `UserConstructionScript`
  (`parent.UserConstructionScript`))