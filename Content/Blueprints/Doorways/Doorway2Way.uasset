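; Two-way doorway Blueprint that switches the player's view between two cameras when interacted with.
; Interaction sets the interact target for all heroes, then calls an empty locked-door hook if locked, or opens a confirm dialog worded for the direction of travel.
; The destination is whichever camera is opposite Camera1 or Camera2; confirming blends to it.
; Confirm and cancel both end in an empty dialog-close hook.
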(event `self.Interactable.OnInteract`
  (bind _ascustom_player_controller (cast `/Game/Blueprints/CustomPlayerController` (`GameplayStatics.GetPlayerController` 0)))
  (`/Game/Blueprints/Interactable.SetInteractTargetForAllHeroes` (`self.Interactable`))
  (if (`self.IsLocked`)
    (`self.OnDoorLocked`)
    (elif (== (`/Game/Blueprints/CustomPlayerController.CurrentCamera` _ascustom_player_controller) (`self.Camera1`))
      (set `self.newCamera` (`self.Camera2`))
      (bind _dialogbox (`/Game/Blueprints/CustomPlayerController.OpenConfirmDialog` _ascustom_player_controller (`self.ConfirmMessage1`) "Yes" "No"))
      (add `/Game/Widgets/ConfirmDialogBox.OnConfirm` _dialogbox (delegate `OnConfirm`))
      (add `/Game/Widgets/ConfirmDialogBox.OnCancel` _dialogbox (delegate `OnCancel`))
      (else
        (set `self.newCamera` (`self.Camera1`))
        (bind _dialogbox_2 (`/Game/Blueprints/CustomPlayerController.OpenConfirmDialog` _ascustom_player_controller (`self.ConfirmMessage2`) "Yes" "No"))
        (add `/Game/Widgets/ConfirmDialogBox.OnConfirm` _dialogbox_2 (delegate `OnConfirm`))
        (add `/Game/Widgets/ConfirmDialogBox.OnCancel` _dialogbox_2 (delegate `OnCancel`))))))

(event `OnCancel`
  (`self.OnCloseConfirmDialog` :!label _label))

(event `OnConfirm`
  (`/Game/Blueprints/CustomPlayerController.SetCurrentCamera` (stale `self.Interactable.OnInteract` _ascustom_player_controller) (`self.newCamera`) 0.5)
  (goto _label))

(fn `OnCloseConfirmDialog`)

(fn `OnDoorLocked`)

(fn `UserConstructionScript`)