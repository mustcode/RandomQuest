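; Party hero character that moves along the X axis in a follow-the-leader line ordered by WorldDataInstance character index.
; The front hero walks to an interact target or, once the player camera stops, catches up to it; others trail behind the hero ahead.
; Interacting opens the controller's skill selection widget in combat mode and tries the chosen skill.
; Reaching an interact target is an empty hook, and skill commands are only printed.
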(event OnInteract(Interactable)
  (bind _ascustom_player_controller (Utilities|Casting|CastToCustomPlayerController (Game|GetPlayerController 0)))
  (bind _selectskillwidget (Default|OpenSelectSkillWidget _ascustom_player_controller))
  (Default|SetSkillsData _selectskillwidget (Class|BaseCharacter|GetSkills) true)
  (EventDispatchers|BindEventtoOnUseSkill _selectskillwidget (delegate Custom|OnUseSkill)))

(event Custom|OnCameraStopped
  (CallFunction|ClearInteractTarget)
  (if (not (Variables|Default|GetIsMoving))
    (Variables|Default|SetIsMoving (CallFunction|IsTooFarfromCamera))))

(event Custom|OnUseSkill
  (params (skill :type Skill%20Structure))
  (Class|BaseCharacter|TryUseSkill (.name (Utilities|Struct|BreakSkill skill))))

(event EventBeginPlay
  (bind _ascustom_player_controller (Utilities|Casting|CastToCustomPlayerController (Game|GetPlayerController 0)))
  (EventDispatchers|BindEventtoOnCameraStopped _ascustom_player_controller (delegate Custom|OnCameraStopped)))

(event EventTick
  (params (DeltaSeconds :type Float%20%28single-precision%29))
  (CallFunction|UpdateMovement))

(event EventOnExecuteSkillCommand
  (params (commands :type Array%20of%20Skill%20Command%20Structures))
  (for _array_element commands
    (Development|PrintString (Utilities|String|ToString(Name) (.command (Utilities|Struct|BreakSkillCommand _array_element))))))

(fn ConstructionScript)

(fn UpdateMovement
  (if (CallFunction|IsFrontMostHero)
    (if (Variables|Default|GetIsMoving)
      (if (CallFunction|HasInteractTarget)
        (bind _target (CallFunction|GetInteractTarget))
        (CallFunction|GotoTarget (Transformation|GetActorLocation _target))
        (if (not (Variables|Default|GetIsMoving))
          (CallFunction|OnReachedInteractTarget))
        (else
          (CallFunction|GotoCamera))))
    (elif (CallFunction|IsTooFarfromHeroinFront)
      (CallFunction|GotoTarget (CallFunction|GetPositionBehindHero (CallFunction|GetHeroinFront))))))

(fn IsTooFarfromCamera
  (bind _ascustom_player_controller (Utilities|Casting|CastToCustomPlayerController (Game|GetPlayerController 0))
    (:then
      (LocalVariables|SetisTooFar (> (Math|Float|Absolute(Float) (- (.X (Math|Vector|BreakVector (Transformation|GetActorLocation (Variables|/Game/Blueprints/CustomPlayerController.CustomPlayerController_C|GetCurrentCamera _ascustom_player_controller)))) (.X (Math|Vector|BreakVector (Transformation|GetActorLocation))))) 1e+02)))
    (:CastFailed
      _))
  (return (LocalVariables|GetisTooFar)))

(fn GotoCamera
  (bind _ascustom_player_controller (Utilities|Casting|CastToCustomPlayerController (Game|GetPlayerController 0)))
  (CallFunction|GotoTarget (Transformation|GetActorLocation (Variables|/Game/Blueprints/CustomPlayerController.CustomPlayerController_C|GetCurrentCamera _ascustom_player_controller))))

(fn GotoTarget
  (params (target :type Vector))
  (bind _returnvalue (Transformation|GetActorLocation))
  (bind _x (Math|Vector|BreakVector target))
  (bind (_x_2 _y _z) (Math|Vector|BreakVector _returnvalue))
  (bind _output_get (LocalVariables|SetDistanceFromTarget (- _x _x_2)))
  (bind _output_get_2 (Variables|Default|SetIsMoving (CallFunction|IsTooFarfromTarget _output_get)))
  (if _output_get_2
    (Pawn|Input|AddMovementInput "1.000000, 0, 0" (Math|Float|Clamp(Float) (LocalVariables|GetDistanceFromTarget) -0.5 0.5) false)
    (if (> (Math|Float|Absolute(Float) (.X (Math|Vector|BreakVector (Transformation|GetVelocity)))) 1.0)
      (Transformation|SetActorRotation (Math|Rotator|FindLookatRotation _returnvalue (Math|Vector|MakeVector _x _y _z))))))

(fn SetInteractTarget
  (params (TargetObject :type Actor%20Object%20Reference))
  (Variables|Default|SetInteractTarget TargetObject)
  (Variables|Default|SetIsMoving true))

(fn OnReachedInteractTarget)

(fn GetInteractTarget
  (return (Variables|Default|GetInteractTarget)))

(fn ClearInteractTarget
  (Variables|Default|SetInteractTarget 0))

(fn HasInteractTarget
  (return (!= (Variables|Default|GetInteractTarget) 0)))

(fn GetHeroinFront
  (bind _asworld_data_instance (Utilities|Casting|CastToWorldDataInstance (Game|GetGameInstance)))
  (bind _returnvalue (Class|WorldDataInstance|GetCharacterIndex _asworld_data_instance (Variables|Default|Getcharacter)))
  (if (== _returnvalue 0)
    (LocalVariables|Setresult 0)
    (else
      (LocalVariables|Setresult (CallFunction|GetHerobyIndex (- _returnvalue 1)))))
  (return (LocalVariables|Getresult)))

(fn GetHerobyIndex
  (params (index :type Integer))
  (LocalVariables|SetindexToCheck index)
  (bind _asworld_data_instance (Utilities|Casting|CastToWorldDataInstance (Game|GetGameInstance)))
  (bind _outactors (Actor|GetAllActorsOfClass "Hero_C"))
  (for _array_element _outactors
    (bind _returnvalue (Class|WorldDataInstance|GetCharacterIndex _asworld_data_instance (Variables|/Script/RandomQuest.BaseCharacter|Getcharacter _array_element)))
    (if (== _returnvalue (LocalVariables|GetindexToCheck))
      (LocalVariables|Setresult _array_element)
      (return (LocalVariables|Getresult))))
  (return (LocalVariables|Getresult)))

(fn GetPositionBehindHero
  (params (heroInFront :type Hero%20Object%20Reference))
  (return (- (Transformation|GetActorLocation heroInFront) (* (Transformation|GetActorForwardVector heroInFront) 5e+01))))

(fn IsFrontMostHero
  (bind _asworld_data_instance (Utilities|Casting|CastToWorldDataInstance (Game|GetGameInstance)))
  (bind _returnvalue (Class|WorldDataInstance|GetCharacterIndex _asworld_data_instance (Variables|Default|Getcharacter)))
  (return (== _returnvalue 0)))

(fn IsTooFarfromHeroinFront
  (if (CallFunction|IsFrontMostHero)
    (LocalVariables|SetisTooFar false)
    (else
      (LocalVariables|SetisTooFar (> (Math|Float|Absolute(Float) (- (.X (Math|Vector|BreakVector (CallFunction|GetPositionBehindHero (CallFunction|GetHeroinFront)))) (.X (Math|Vector|BreakVector (Transformation|GetActorLocation))))) 3e+01))))
  (return (LocalVariables|GetisTooFar)))

(fn IsTooFarfromTarget
  (params (distanceFromTarget :type Float%20%28single-precision%29))
  (bind _returnvalue (Math|Float|Absolute(Float) distanceFromTarget))
  (if (CallFunction|IsFrontMostHero)
    (bind _output_get (LocalVariables|SetdistanceLimit 5e+01))
    (LocalVariables|SetisTooFar (> _returnvalue _output_get))
    (else
      (bind _output_get_2 (LocalVariables|SetdistanceLimit 35.0))
      (LocalVariables|SetisTooFar (> _returnvalue _output_get_2))))
  (return (LocalVariables|GetisTooFar)))