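; Gate connection that links the current dungeon to a named town.
; It supplies both endpoints by querying the WorldDataInstance game instance: the destination is the town looked up by the Destination name, and the current location is the active dungeon.
; The construction script only runs the parent's.
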(fn `GetCurrentLocation`
  (returns (location :type "LocationObject Object Reference"))
  (bind _asworld_data_instance (cast `WorldDataInstance` (`GameplayStatics.GetGameInstance`)))
  (return (`WorldDataInstance.GetCurrentDungeon` _asworld_data_instance)))

(fn `GetDestinationLocation`
  (returns (location :type "LocationObject Object Reference"))
  (bind _asworld_data_instance (cast `WorldDataInstance` (`GameplayStatics.GetGameInstance`)))
  (return (`WorldDataInstance.GetTownByName` _asworld_data_instance (`self.destination`))))

(fn `UserConstructionScript`
  (`parent.UserConstructionScript`))