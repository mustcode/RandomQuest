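; GateConnection is an interactable gate that sends the player to an entrance in another town.
; On interact it opens a confirm dialog through CustomPlayerController, then asks CustomGameMode to travel to its Destination and Entrance.
; The construction script labels the gate's text with the destination.
; AddConnection registers a given gate as a link from the current town to the destination, resolving both through WorldDataInstance.
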(event `self.ReceiveBeginPlay`
  (add `/Game/Blueprints/Interactable.OnInteract` (`self.Interactable`) (delegate `OnInteract`)))

(event `OnInteract`
  (bind _ascustom_player_controller (cast `/Game/Blueprints/CustomPlayerController` (`GameplayStatics.GetPlayerController` 0)))
  (bind _dialogbox (`/Game/Blueprints/CustomPlayerController.OpenConfirmDialog` _ascustom_player_controller (`KismetTextLibrary.Conv_StringToText` (`KismetStringLibrary.BuildString_Name` "" "Travel To " (`self.destination`) "?")) "Yes" "No"))
  (add `/Game/Widgets/ConfirmDialogBox.OnConfirm` _dialogbox (delegate `OnConfirm`)))

(event `OnConfirm`
  (`self.TravelToDestination`))

(fn `AddConnection`
  (params (gate :type "/Game/Blueprints/Gates/Gate Object Reference"))
  (bind _location (`self.GetCurrentLocation`))
  (bind _location_2 (`self.GetDestinationLocation`))
  (`LocationObject.AddConnection` _location (`/Game/Blueprints/Gates/Gate.gateName` gate) _location_2 (`self.entrance`)))

(fn `GetCurrentLocation`
  (returns (location :type "LocationObject Object Reference"))
  (bind _asworld_data_instance (cast `WorldDataInstance` (`GameplayStatics.GetGameInstance`)))
  (return (`WorldDataInstance.GetCurrentTown` _asworld_data_instance)))

(fn `GetDestinationLocation`
  (returns (location :type "LocationObject Object Reference"))
  (bind _asworld_data_instance (cast `WorldDataInstance` (`GameplayStatics.GetGameInstance`)))
  (return (`WorldDataInstance.GetTownByName` _asworld_data_instance (`self.destination`))))

(fn `TravelToDestination`
  (returns (result :type Boolean))
  (bind _ascustom_game_mode (cast `/Game/Blueprints/CustomGameMode` (`GameplayStatics.GetGameMode`)))
  (`/Game/Blueprints/CustomGameMode.TravelToLocation` _ascustom_game_mode (`self.destination`) (`self.entrance`))
  (return true))

(fn `UserConstructionScript`
  (`TextRenderComponent.SetText` (`self.TextRender`) (`KismetStringLibrary.Concat_StrStr` "Travel to " (`KismetStringLibrary.Conv_NameToString` (`self.destination`)))))