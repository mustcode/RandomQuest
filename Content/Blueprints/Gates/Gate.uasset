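; Gate actor that marks a named gate in a town and sets up the camera when it is the world's current gate.
; On BeginPlay, if the game instance's current gate matches its name or is "None", it switches the player controller to its camera and positions it.
; AddGate registers the gate with the current town if absent, then adds itself to each connection.
; The construction script displays the gate name as text.
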(event `self.ReceiveBeginPlay`
  (bind _asworld_data_instance (cast `WorldDataInstance` (`GameplayStatics.GetGameInstance`)))
  (bind _currentgate (`WorldDataInstance.currentGate` _asworld_data_instance))
  (if (or (== _currentgate (`self.gateName`)) (== _currentgate "None"))
    (bind _ascustom_player_controller (cast `/Game/Blueprints/CustomPlayerController` (`GameplayStatics.GetPlayerController` 0)))
    (`/Game/Blueprints/CustomPlayerController.SetCurrentCamera` _ascustom_player_controller (`self.Camera`) 0.0)
    (`KismetSystemLibrary.PrintString` (`KismetStringLibrary.Conv_NameToString` (`self.gateName`)))
    (if (!= (`self.Camera`) null)
      (`SceneComponent.K2_SetWorldLocationAndRotation` (`self.Camera`) (`self.CameraPosition`) (`self.CameraDirection`) false))))

(fn `AddGate`
  (bind _location (`self.GetCurrentLocation`))
  (if (not (`LocationObject.HasGate` _location (`self.gateName`)))
    (`LocationObject.AddGate` _location (`self.gateName`))
    (for _array_element (`self.connections`)
      (`/Game/Blueprints/Gates/GateConnection.AddConnection` _array_element self))))

(fn `GetCurrentLocation`
  (returns (location :type "LocationObject Object Reference"))
  (bind _asworld_data_instance (cast `WorldDataInstance` (`GameplayStatics.GetGameInstance`)))
  (return (`WorldDataInstance.GetCurrentTown` _asworld_data_instance)))

(fn `UserConstructionScript`
  (`TextRenderComponent.SetText` (`self.TextRender`) (`KismetStringLibrary.Conv_NameToString` (`self.gateName`))))