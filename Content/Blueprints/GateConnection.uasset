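; GateConnection is a clickable or tappable travel point that links a gate to another town.
; Releasing it opens a confirm dialog through the custom player controller, and confirming asks the game mode to travel to TownName at Entrance.
; The construction script labels its text render with the destination.
; AddConnection records the link from a given gate to that town and entrance on the current town in the game instance's world data.
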(event `self.ReceiveActorOnReleased`
  (bind _ascustom_player_controller (cast `/Game/Blueprints/CustomPlayerController` (`GameplayStatics.GetPlayerController` 0)))
  (bind _dialogbox (`/Game/Blueprints/CustomPlayerController.OpenConfirmDialog` _ascustom_player_controller (`KismetTextLibrary.Conv_StringToText` (`KismetStringLibrary.BuildString_Name` "" "Travel To " (`self.townName`) "?")) "Yes" "No"))
  (add `/Game/Widgets/ConfirmDialogBox.OnConfirm` _dialogbox (delegate `OnConfirm`)))

(event `OnConfirm`
  (bind _ascustom_game_mode (cast `/Game/Blueprints/CustomGameMode` (`GameplayStatics.GetGameMode`)))
  (`/Game/Blueprints/CustomGameMode.TravelToTown` _ascustom_game_mode (`self.townName`) (`self.entrance`)))

(fn `AddConnection`
  (params (gate :type "/Game/Blueprints/Gates/Gate Object Reference"))
  (bind _asworld_data_instance (cast `WorldDataInstance` (`GameplayStatics.GetGameInstance`)))
  (`LocationObject.AddConnection` (`WorldDataInstance.GetCurrentTown` _asworld_data_instance) (`/Game/Blueprints/Gates/Gate.gateName` gate) (`WorldDataInstance.GetTownByName` _asworld_data_instance (`self.townName`)) (`self.entrance`)))

(fn `UserConstructionScript`
  (`TextRenderComponent.SetText` (`self.TextRender`) (`KismetStringLibrary.Concat_StrStr` "Travel to " (`KismetStringLibrary.Conv_NameToString` (`self.townName`)))))