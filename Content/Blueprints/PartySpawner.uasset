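; PartySpawner places the player's party of heroes in the level at the gate recorded in the WorldDataInstance game instance.
; SpawnHeroesInParty finds all SpawnPoint actors and keeps those whose gate name matches CurrentGate and whose index is below the party size.
; At each, it spawns a Hero with a default controller, initializes it with that index's character data and attaches a new Weapon to its right-hand socket.
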(event EventBeginPlay)

(event EventTick
  (params (DeltaSeconds :type Float%20%28single-precision%29)))

(fn SpawnHeroesinParty
  (bind _asworld_data_instance (Utilities|Casting|CastToWorldDataInstance (Game|GetGameInstance)))
  (bind _output_get (LocalVariables|SetPartySize (Class|WorldDataInstance|GetPartySize _asworld_data_instance)))
  (if (> _output_get 0)
    (LocalVariables|SetCurrentGate (Variables|/Script/RandomQuest.WorldDataInstance|GetcurrentGate _asworld_data_instance))
    (bind _outactors (Actor|GetAllActorsOfClass "/Game/Blueprints/SpawnPoint.SpawnPoint_C"))
    (for _array_element _outactors
      (if (and (< (Variables|/Game/Blueprints/SpawnPoint.SpawnPoint_C|Getindex _array_element) (LocalVariables|GetPartySize)) (Utilities|Name|Equal(Name) (LocalVariables|GetCurrentGate) (Variables|/Game/Blueprints/Gates/Gate.Gate_C|GetgateName (Variables|/Game/Blueprints/SpawnPoint.SpawnPoint_C|Getgate _array_element))))
        (bind _returnvalue (Game|SpawnActorfromClass "/Game/Blueprints/Hero.Hero_C" (Transformation|GetActorTransform _array_element) "AlwaysSpawn" 0 0))
        (Pawn|SpawnDefaultController _returnvalue)
        (Class|BaseCharacter|Init _returnvalue (Class|WorldDataInstance|GetCharacterbyIndex _asworld_data_instance (Variables|/Game/Blueprints/SpawnPoint.SpawnPoint_C|Getindex _array_element)))
        (bind _returnvalue_2 (Game|SpawnActorfromClass "/Game/Blueprints/Weapons/Weapon.Weapon_C" (Math|Transform|MakeTransform "0, 0, 0") "AlwaysSpawn" 0 0))
        (Class|Actor|AttachRootComponentto _returnvalue_2 (Variables|/Script/Engine.Character|GetMesh _returnvalue) "hand_r" "SnapToTarget" true)))))