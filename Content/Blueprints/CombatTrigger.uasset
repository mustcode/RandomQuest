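; CombatTrigger is a component that starts a combat encounter when a Hero overlaps the trigger volume that owns it.
; On BeginPlay it binds to the owning TriggerBase's begin-overlap event.
; If combat is not already active, the overlap registers each Enemy from its SpawnPoints with CustomGameMode through AddEnemy.
; An AlreadyTriggered flag then blocks further triggering, though a failed Enemy cast exits before setting it.
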(event `self.ReceiveBeginPlay`
  (bind _astrigger_base (cast `TriggerBase` (`self.GetOwner`)))
  (add `Actor.OnActorBeginOverlap` _astrigger_base (delegate `OnActorBeginOverlapped`)))

(event `OnActorBeginOverlapped`
  (params (OtherActor :type "Actor Object Reference"))
  (if (and (not (`self.alreadyTriggered`)) (not (`self.IsInCombat`)))
    (if (`KismetMathLibrary.ClassIsChildOf` (`GameplayStatics.GetObjectClass` OtherActor) "/Game/Blueprints/Hero.Hero_C")
      (bind _ascustom_game_mode (cast `/Game/Blueprints/CustomGameMode` (`GameplayStatics.GetGameMode`)))
      (for _array_element (`self.SpawnPoints`)
        (bind _asenemy (cast `/Game/Blueprints/Enemy` (`/Game/Blueprints/RandomActorSpawnPoint.GetSpawnedActor` _array_element)))
        (`/Game/Blueprints/CustomGameMode.AddEnemy` _ascustom_game_mode _asenemy))
      (set `self.alreadyTriggered` true))))

(fn `IsInCombat`
  (returns (result :type Boolean))
  (bind _ascustom_game_mode (cast `/Game/Blueprints/CustomGameMode` (`GameplayStatics.GetGameMode`)))
  (return (`/Game/Blueprints/CustomGameMode.IsInCombat` _ascustom_game_mode)))