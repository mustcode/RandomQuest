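; CameraScrollBounds is a component that confines its owning actor, by name a scrolling camera, to an axis-aligned box set by min and max limits on X, Y and Z.
; KeepInBound checks the owner's location against the limits and, if any axis is outside, clamps all three and sets the location without sweeping.
; Tick and BeginPlay are disabled stubs, so bounds apply only when KeepInBound is called externally.
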(event EventTick
  (params (DeltaSeconds :type Float%20%28single-precision%29)))

(event EventBeginPlay)

(fn KeepinBound
  (bind _output_get (LocalVariables|Setowner (Components|GetOwner)))
  (if (Math|Boolean|ORBoolean (> (.X (Math|Vector|BreakVector (Transformation|GetActorLocation _output_get))) (Variables|Default|GetmaxX)) (< (.X (Math|Vector|BreakVector (Transformation|GetActorLocation _output_get))) (Variables|Default|GetminX)) (> (.Y (Math|Vector|BreakVector (Transformation|GetActorLocation _output_get))) (Variables|Default|GetmaxY)) (< (.Y (Math|Vector|BreakVector (Transformation|GetActorLocation _output_get))) (Variables|Default|GetminY)) (> (.Z (Math|Vector|BreakVector (Transformation|GetActorLocation _output_get))) (Variables|Default|GetmaxZ)) (< (.Z (Math|Vector|BreakVector (Transformation|GetActorLocation _output_get))) (Variables|Default|GetminZ)))
    (Transformation|SetActorLocation (LocalVariables|Getowner) (Math|Vector|MakeVector (Math|Float|Clamp(Float) (.X (Math|Vector|BreakVector (Transformation|GetActorLocation _output_get))) (Variables|Default|GetminX) (Variables|Default|GetmaxX)) (Math|Float|Clamp(Float) (.Y (Math|Vector|BreakVector (Transformation|GetActorLocation _output_get))) (Variables|Default|GetminY) (Variables|Default|GetmaxY)) (Math|Float|Clamp(Float) (.Z (Math|Vector|BreakVector (Transformation|GetActorLocation _output_get))) (Variables|Default|GetminZ) (Variables|Default|GetmaxZ))) false)))