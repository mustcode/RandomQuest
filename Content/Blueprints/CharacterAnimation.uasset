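; CharacterAnimation is a Blueprint that holds pending action names in an ActionStack array, presumably for character animation.
; PushAction appends to the end and PopAction removes and returns the first element, so the array behaves as a FIFO queue despite its name.
; HasAction reports whether entries remain, and PeekAction uses it to return the front name or "None"; PopAction has no empty check.
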(event EventBeginPlay)

(event EventTick
  (params (DeltaSeconds :type Float%20%28single-precision%29)))

(fn PushAction
  (params (actionName :type Name))
  (Utilities|Array|Add (Variables|Default|GetActionStack) actionName))

(fn PopAction
  (LocalVariables|Setresult (Utilities|Array|Get(acopy) (Variables|Default|GetActionStack)))
  (Utilities|Array|RemoveIndex (Variables|Default|GetActionStack))
  (return (LocalVariables|Getresult)))

(fn HasAction
  (return (> (Utilities|Array|Length (Variables|Default|GetActionStack)) 0)))

(fn PeekAction
  (if (CallFunction|HasAction)
    (return (Utilities|Array|Get(acopy) (Variables|Default|GetActionStack)))
    (else
      (return ""))))