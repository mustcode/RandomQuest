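; Player controller that drives drag-to-scroll cameras and owns the confirm and conversation dialog widgets.
; Holding left mouse pans the current camera by mouse delta, mapping axes by the SideScroll flag and clamping through its CameraScrollBounds component.
; Left click also advances a visible conversation.
; SetCurrentCamera blends the view to a new camera and caches its bounds; helpers open dialogs and report their visibility.
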(event EventBeginPlay)

(event EventTick
  (params (DeltaSeconds :type Float%20%28single-precision%29))
  (Variables|Default|SetdeltaSeconds DeltaSeconds))

(event Input|MouseEvents|MouseY
  (params (AxisValue :type Float%20%28single-precision%29))
  (bind (_deltax _deltay) (Class|PlayerController|GetInputMouseDelta))
  (bind _deltaseconds (Variables|Default|GetdeltaSeconds))
  (bind _deltaseconds_2 (Variables|Default|GetdeltaSeconds))
  (bind _returnvalue (* _deltay -3e+02))
  (bind _returnvalue_2 (* _deltax -3e+02))
  (bind _returnvalue_3 (* _returnvalue _deltaseconds))
  (bind _returnvalue_4 (* _deltaseconds_2 _returnvalue_2))
  (if (and (Variables|Default|Getdragging) (!= (Variables|Default|GetcameraBound) 0))
    (if (Variables|/Game/Blueprints/CameraScrollBounds.CameraScrollBounds_C|GetsideScroll (Variables|Default|GetcameraBound))
      (CallFunction|UpdateCameraPosition (Math|Vector|MakeVector _returnvalue_4 _returnvalue_3 0.0))
      (else
        (CallFunction|UpdateCameraPosition (Math|Vector|MakeVector _returnvalue_3 _returnvalue_4 0.0))))))

(event Input|MouseEvents|MouseX
  (params (AxisValue :type Float%20%28single-precision%29))
  (bind (_deltax _deltay) (Class|PlayerController|GetInputMouseDelta))
  (bind _deltaseconds (Variables|Default|GetdeltaSeconds))
  (bind _deltaseconds_2 (Variables|Default|GetdeltaSeconds))
  (bind _returnvalue (* _deltay -3e+02))
  (bind _returnvalue_2 (* _deltax -3e+02))
  (bind _returnvalue_3 (* _returnvalue _deltaseconds))
  (bind _returnvalue_4 (* _deltaseconds_2 _returnvalue_2))
  (if (and (Variables|Default|Getdragging) (!= (Variables|Default|GetcameraBound) 0))
    (if (Variables|/Game/Blueprints/CameraScrollBounds.CameraScrollBounds_C|GetsideScroll (Variables|Default|GetcameraBound))
      (CallFunction|UpdateCameraPosition (Math|Vector|MakeVector _returnvalue_4 _returnvalue_3 0.0))
      (else
        (CallFunction|UpdateCameraPosition (Math|Vector|MakeVector _returnvalue_3 _returnvalue_4 0.0))))))

(event Input|MouseEvents|LeftMouseButton
  (:Pressed
    (Variables|Default|Setdragging true)
    (CallFunction|AdvanceConversation))
  (:Released
    (Variables|Default|Setdragging false)))

(fn ConstructionScript)

(fn OpenConfirmDialog
  (params (QuestionText :type Text) (ConfirmText :type Text) (CancelText :type Text))
  (bind _returnvalue (UserInterface|CreateWidget "/Game/Widgets/ConfirmDialogBox.ConfirmDialogBox_C"))
  (Variables|Default|SetConfirmDIalog _returnvalue)
  (Utilities|FlowControl|Sequence
    (:then_0
      (Variables|/Game/Widgets/ConfirmDialogBox.ConfirmDialogBox_C|SetQuestionText (Variables|Default|GetConfirmDIalog) QuestionText))
    (:then_1
      (Variables|/Game/Widgets/ConfirmDialogBox.ConfirmDialogBox_C|SetConfirmText (Variables|Default|GetConfirmDIalog) ConfirmText))
    (:then_2
      (Variables|/Game/Widgets/ConfirmDialogBox.ConfirmDialogBox_C|SetCancelText (Variables|Default|GetConfirmDIalog) CancelText))
    (:then_3
      (UserInterface|Viewport|AddtoViewport (Variables|Default|GetConfirmDIalog) 0)
      (return (Variables|Default|GetConfirmDIalog)))))

(fn CloseConfirmDialog
  (Widget|RemovefromParent (Variables|Default|GetConfirmDIalog)))

(fn IsConfirmDialogVisible
  (return (CallFunction|IsWidgetVisible (Variables|Default|GetConfirmDIalog))))

(fn SetCurrentCamera
  (params (CameraActor :type Camera%20Actor%20Object%20Reference) (blendTIme :type Float%20%28single-precision%29 :default 0.0))
  (bind _output_get (Variables|Default|SetCurrentCamera CameraActor))
  (Game|Player|SetViewTargetwithBlend (Game|GetPlayerController 0) _output_get blendTIme "VTBlend_EaseOut" 2.5 false)
  (Variables|Default|SetcameraBound (Utilities|Array|Get(acopy) (Actor|GetComponentsByClass (Variables|Default|GetCurrentCamera) "/Game/Blueprints/CameraScrollBounds.CameraScrollBounds_C")))
  (Default|CallOnCameraMoved))

(fn OpenConversationDialog
  (params (DialogOwner :type Actor%20Object%20Reference))
  (bind _returnvalue (UserInterface|CreateWidget "/Game/Widgets/ConversationDialog.ConversationDialog_C" 0 DialogOwner))
  (bind _output_get (Variables|Default|SetConversationDialog _returnvalue))
  (Default|HideChoices _output_get)
  (UserInterface|Viewport|AddtoViewport (Variables|Default|GetConversationDialog) 0)
  (return (Variables|Default|GetConversationDialog)))

(fn AdvanceConversation
  (if (!= (Variables|Default|GetConversationDialog) 0)
    (if (Widget|IsVisible (Variables|Default|GetConversationDialog))
      (Default|AdvanceConversation (Variables|Default|GetConversationDialog)))))

(fn UpdateCameraPosition
  (params (DeltaLocation :type Vector :default "0, 0, 0"))
  (if (> (Math|Vector|VectorLengthSquared DeltaLocation) 0.1)
    (Transformation|AddRelativeLocation (Variables|Default|GetCurrentCamera) DeltaLocation false)
    (Default|KeepinBound (Variables|Default|GetcameraBound))
    (Default|CallOnCameraMoved)))

(fn IsWidgetVisible
  (params (widget :type Widget%20Object%20Reference))
  (if (!= widget 0)
    (LocalVariables|Setresult (Widget|IsVisible widget))
    (else
      (LocalVariables|Setresult false)))
  (return (LocalVariables|Getresult)))

(fn IsConversationDialogVisible
  (return (CallFunction|IsWidgetVisible (Variables|Default|GetConversationDialog))))

(fn IsAnyDialogBoxVisible
  (return (or (CallFunction|IsConfirmDialogVisible) (CallFunction|IsConversationDialogVisible))))