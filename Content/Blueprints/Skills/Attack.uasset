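; Attack is a skill actor that deals damage from its Activator to a set of target actors.
; On BeginPlay it sets a three-second lifespan, waits half a second, then loops over TargetActors.
; Each target that casts to BaseCharacter receives ApplyDamage with DamageAmount and the Activator as originator, followed by a debug print.
; The construction script only calls its parent.
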(event `self.ReceiveBeginPlay`
  (`self.SetLifeSpan` 3.0)
  (`KismetSystemLibrary.Delay` 0.5)
  (for _array_element (`self.targetActors`)
    (bind _asbase_character (cast `BaseCharacter` _array_element))
    (bind _asbase_character_2 (cast `BaseCharacter` (`self.activator`)))
    (`BaseCharacter.ApplyDamage` _asbase_character _asbase_character_2 (`self.damageAmount`) "None")
    (`KismetSystemLibrary.PrintString` "Applying Damage")))

(fn `UserConstructionScript`
  (`parent.UserConstructionScript`))