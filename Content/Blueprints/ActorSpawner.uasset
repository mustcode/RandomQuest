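; ActorSpawner is a utility Blueprint that spawns actors by name from a configured list.
; SpawnActor searches ActorsList for an entry with a matching Name and spawns its ActorClass at the given transform, always spawning regardless of collision.
; It returns the spawned actor, or prints a red on-screen error when no entry matches.
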(event `self.ReceiveTick`
  (params (DeltaSeconds :type "Float (single-precision)")))

(event `self.ReceiveBeginPlay`)

(fn `SpawnActor`
  (params (name :type Name) (transform :type "Transform Structure"))
  (returns (actor :type "Actor Object Reference"))
  (for _array_element (`self.ActorsList`)
    (bind (_name _actorclass) (break `/Game/Blueprints/NameClassPair` _array_element))
    (if (== name _name)
      (bind _returnvalue (`|SpawnActorFromClass` _actorclass transform "AlwaysSpawn" "OverrideRootScale"))
      (return _returnvalue)))
  (`KismetSystemLibrary.PrintString` (`KismetTextLibrary.Conv_TextToString` (`|FormatText` "Actor \"{name}\" not found" (`KismetTextLibrary.Conv_NameToText` name))) true true (struct :`R` 1.0 :`A` 1.0) 5.0))