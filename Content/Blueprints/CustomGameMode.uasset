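; Game mode for a party-based game with heroes, gates and combat, acting as a function library over the WorldDataInstance game instance.
; Level travel stores the entrance as CurrentGate, which selects the spawn points for party heroes with attached weapons and the gate that sets up the camera.
; It also moves living heroes to exit points by party index and forwards ability tests and random recruitment to the game instance.
; Combat state is simply a non-empty Enemies list.
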(event EventBeginPlay)

(event EventTick
  (params (DeltaSeconds :type Float%20%28single-precision%29)))

(fn ConstructionScript)

(fn TraveltoLocation
  (params (DestinationName :type Name :default "None") (EntranceName :type Name :default "None"))
  (bind _asworld_data_instance (Utilities|Casting|CastToWorldDataInstance (Game|GetGameInstance)))
  (Variables|/Script/RandomQuest.WorldDataInstance|SetcurrentGate _asworld_data_instance EntranceName)
  (Game|OpenLevel(byName) DestinationName))

(fn AbilityTest
  (params (heroIndex :type Integer) (attribute :type Name) (difficulty :type Integer))
  (bind _asworld_data_instance (Utilities|Casting|CastToWorldDataInstance (Game|GetGameInstance)))
  (bind (_result _returnvalue) (Class|WorldDataInstance|AbilityTest _asworld_data_instance heroIndex attribute difficulty))
  (return _result _returnvalue))

(fn LogGameMessage
  (params (message :type String))
  (Development|PrintString message))

(fn GetHerobyIndex
  (params (Index :type Integer))
  (LocalVariables|SetindexToCheck Index)
  (bind _asworld_data_instance (Utilities|Casting|CastToWorldDataInstance (Game|GetGameInstance)))
  (bind _outactors (Actor|GetAllActorsOfClass "/Game/Blueprints/Hero.Hero_C"))
  (for _array_element _outactors
    (if (not (Class|BaseCharacter|IsDead _array_element))
      (bind _returnvalue (Class|WorldDataInstance|GetCharacterIndex _asworld_data_instance (Variables|/Script/RandomQuest.BaseCharacter|Getcharacter _array_element)))
      (if (== _returnvalue (LocalVariables|GetindexToCheck))
        (LocalVariables|Setresult _array_element)
        (return (LocalVariables|Getresult)))))
  (return (LocalVariables|Getresult)))

(fn AddRandomHerotoParty
  (bind _asworld_data_instance (Utilities|Casting|CastToWorldDataInstance (Game|GetGameInstance)))
  (bind _returnvalue (Class|WorldDataInstance|CreateCharacter _asworld_data_instance))
  (Class|WorldDataInstance|AddCharactertoParty _asworld_data_instance _returnvalue))

(fn AddEnemy
  (params (Enemy :type Enemy%20Object%20Reference))
  (Utilities|Array|Add (Variables|Default|GetEnemies) Enemy))

(fn ClearEnemies
  (Utilities|Array|Clear (Variables|Default|GetEnemies)))

(fn IsinCombat
  (return (> (Utilities|Array|Length (Variables|Default|GetEnemies)) 0)))

(fn RemoveEnemy
  (params (enemy :type Enemy%20Object%20Reference))
  (bind _returnvalue (Utilities|Array|RemoveItem (Variables|Default|GetEnemies) enemy))
  (return _returnvalue))

(fn SpawnHeroesinParty
  (bind _asworld_data_instance (Utilities|Casting|CastToWorldDataInstance (Game|GetGameInstance)))
  (bind _output_get (LocalVariables|SetPartySize (Class|WorldDataInstance|GetPartySize _asworld_data_instance)))
  (if (> _output_get 0)
    (LocalVariables|SetCurrentGate (Variables|/Script/RandomQuest.WorldDataInstance|GetcurrentGate _asworld_data_instance))
    (bind _outactors (Actor|GetAllActorsOfClass "/Game/Blueprints/SpawnPoint.SpawnPoint_C"))
    (for _array_element _outactors
      (if (and (< (Variables|/Game/Blueprints/SpawnPoint.SpawnPoint_C|Getindex _array_element) (LocalVariables|GetPartySize)) (Utilities|Name|Equal(Name) (LocalVariables|GetCurrentGate) (Variables|/Game/Blueprints/Gates/Gate.Gate_C|GetgateName (Variables|/Game/Blueprints/SpawnPoint.SpawnPoint_C|Getgate _array_element))))
        (bind _returnvalue (Game|SpawnActorfromClass "/Game/Blueprints/Hero.Hero_C" (Transformation|GetActorTransform _array_element) "AlwaysSpawn" 0 0))
        (Pawn|SpawnDefaultController _returnvalue)
        (Class|BaseCharacter|Init _returnvalue (Class|WorldDataInstance|GetCharacterbyIndex _asworld_data_instance (Variables|/Game/Blueprints/SpawnPoint.SpawnPoint_C|Getindex _array_element)))
        (bind _returnvalue_2 (Game|SpawnActorfromClass "/Game/Blueprints/Weapons/Weapon.Weapon_C" (Math|Transform|MakeTransform "0, 0, 0") "AlwaysSpawn" 0 0))
        (Class|Actor|AttachRootComponentto _returnvalue_2 (Variables|/Script/Engine.Character|GetMesh _returnvalue) "hand_r" "SnapToTarget" true)))))

(fn MoveHeroestoExitPoints
  (params (ExitPoints :type Array%20of%20Exit%20Point%20Object%20References))
  (bind _asworld_data_instance (Utilities|Casting|CastToWorldDataInstance (Game|GetGameInstance)))
  (bind _outactors (Actor|GetAllActorsOfClass "/Game/Blueprints/Hero.Hero_C"))
  (for _array_element _outactors
    (if (not (Class|BaseCharacter|IsDead _array_element))
      (bind _returnvalue (Class|WorldDataInstance|GetCharacterIndex _asworld_data_instance (Variables|/Script/RandomQuest.BaseCharacter|Getcharacter _array_element)))
      (Transformation|SetActorTransform _array_element (Transformation|GetActorTransform (Utilities|Array|Get(acopy) ExitPoints _returnvalue))))))

(fn AssignRandomGate
  (bind _outactors (Actor|GetAllActorsOfClass "/Game/Blueprints/Gates/Gate.Gate_C"))
  (bind _asworld_data_instance (Utilities|Casting|CastToWorldDataInstance (Game|GetGameInstance)))
  (Variables|/Script/RandomQuest.WorldDataInstance|SetcurrentGate _asworld_data_instance (Variables|/Game/Blueprints/Gates/Gate.Gate_C|GetgateName (Utilities|Array|Get(acopy) _outactors (Math|Random|RandomInteger (Utilities|Array|Length _outactors))))))

(fn SetCameratoGate
  (bind _asworld_data_instance (Utilities|Casting|CastToWorldDataInstance (Game|GetGameInstance)))
  (bind _outactors (Actor|GetAllActorsOfClass "/Game/Blueprints/Gates/Gate.Gate_C"))
  (for _array_element _outactors
    (if (Utilities|Name|Equal(Name) (Variables|/Script/RandomQuest.WorldDataInstance|GetcurrentGate _asworld_data_instance) (Variables|/Game/Blueprints/Gates/Gate.Gate_C|GetgateName _array_element))
      (Default|SetupCamera _array_element))))