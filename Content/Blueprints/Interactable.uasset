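; Interactable is a component that makes its owning actor a click target for Hero interaction.
; On initialization it binds to the owner's clicked and released events.
; A click sets a Clicked flag; a following release clears it and calls SetInteractTarget with the owner on every Hero actor, found through GetAllActorsOfClass.
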(event `self.ReceiveTick`
  (params (DeltaSeconds :type "Float (single-precision)")))

(event `self.ReceiveInitializeComponent`
  (bind _returnvalue (`self.GetOwner`))
  (add `Actor.OnReleased` _returnvalue (delegate `OnActorReleased`))
  (add `Actor.OnClicked` _returnvalue (delegate `OnActorClicked`)))

(event `OnActorClicked`
  (set `self.clicked` true))

(event `OnActorReleased`
  (if (`self.clicked`)
    (set `self.clicked` false)
    (bind _outactors (`GameplayStatics.GetAllActorsOfClass` "/Game/Blueprints/Hero.Hero_C"))
    (for _array_element _outactors
      (`/Game/Blueprints/Hero.SetInteractTarget` _array_element (`self.GetOwner`)))))